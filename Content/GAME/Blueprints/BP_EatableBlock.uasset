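; BP_EatableBlock is a block actor that can be eaten, removing it from the level.
; A sphere overlap sets DetectPlayer while BP_ThirdPersonCharacter is inside.
; TryEating calls EatStageUpdate on the BP_GameInstance cached at BeginPlay, then destroys the block unless EatFull is set after that update.
; TryEating does not check DetectPlayer itself.
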(event OnComponentBeginOverlap(Sphere)
  (params (OverlappedComponent :type Primitive%20Component%20Object%20Reference) (OtherActor :type Actor%20Object%20Reference) (OtherComp :type Primitive%20Component%20Object%20Reference) (OtherBodyIndex :type Integer) (bFromSweep :type Boolean) (SweepResult :type Hit%20Result%20Structure%20%28by%20ref%29))
  (Utilities|Casting|CastToBP_ThirdPersonCharacter OtherActor)
  (Variables|Default|SetDetectPlayer true))

(event OnComponentEndOverlap(Sphere)
  (params (OverlappedComponent :type Primitive%20Component%20Object%20Reference) (OtherActor :type Actor%20Object%20Reference) (OtherComp :type Primitive%20Component%20Object%20Reference) (OtherBodyIndex :type Integer))
  (Utilities|Casting|CastToBP_ThirdPersonCharacter OtherActor)
  (Variables|Default|SetDetectPlayer false))

(event EventBeginPlay
  (bind _asbp_game_instance (Utilities|Casting|CastToBP_GameInstance (Game|GetGameInstance)))
  (Variables|Default|SetAs%20BP%20Game%20Instance _asbp_game_instance))

(event Collision|EventActorBeginOverlap
  (params (OtherActor :type Actor%20Object%20Reference)))

(event EventTick
  (params (DeltaSeconds :type Float%20%28single-precision%29)))

(event EventTryEating
  (bind _as_bp_game_instance (Variables|Default|GetAs%20BP%20Game%20Instance))
  (Default|EatStageUpdate _as_bp_game_instance)
  (if (not (Variables|/Game/GAME/Blueprints/BP_GameInstance.BP_GameInstance_C|GetEatFull _as_bp_game_instance))
    (Actor|DestroyActor)))

(fn ConstructionScript)