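; BP_RuleBreak_JUMP is an edible actor that unlocks jumping when eaten.
; On BeginPlay it casts the game instance to BP_GameInstance and caches the reference.
; Its TryEating event sets JumpUnlock to true on that game instance, then destroys the actor.
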(event EventBeginPlay
  (|CallParentFunction)
  (bind _asbp_game_instance (Utilities|Casting|CastToBP_GameInstance (Game|GetGameInstance)))
  (Variables|Default|SetAs%20BP%20Game%20Instance_0 _asbp_game_instance))

(event Collision|EventActorBeginOverlap
  (params (OtherActor :type Actor%20Object%20Reference))
  (|CallParentFunction OtherActor) ; This node is disabled and will not be called.\nDrag off pins to build functionality.
)

(event EventTick
  (params (DeltaSeconds :type Float%20%28single-precision%29))
  (|CallParentFunction DeltaSeconds) ; This node is disabled and will not be called.\nDrag off pins to build functionality.
)

(event EventTryEating
  (Variables|/Game/GAME/Blueprints/BP_GameInstance.BP_GameInstance_C|SetJumpUnlock (Variables|Default|GetAs%20BP%20Game%20Instance_0) true)
  (Actor|DestroyActor))

(fn ConstructionScript
  (|CallParentFunction))